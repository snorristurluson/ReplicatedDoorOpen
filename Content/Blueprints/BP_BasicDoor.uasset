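; BP_BasicDoor is a simple door Blueprint that snaps a Door component between closed and open rotations.
; Open and Close events set the relative rotation instantly to a 90-degree swing or back to zero, with no interpolation.
; A separate UpdateDoorState function applies the same rotations from the IsOpen flag, which neither event sets.
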(event `/Game/Blueprints/Openable.Open`
  (`SceneComponent.K2_SetRelativeRotation` (`self.Door`) (struct :`Yaw` 90.0) false false))

(event `/Game/Blueprints/Openable.Close`
  (`SceneComponent.K2_SetRelativeRotation` (`self.Door`) (struct) false false))

(fn `Update Door State`
  (if (`self.Is Open?`)
    (`SceneComponent.K2_SetRelativeRotation` (`self.Door`) (struct :`Yaw` 90.0) false false)
    (else
      (`SceneComponent.K2_SetRelativeRotation` (`self.Door`) (struct) false false))))

(fn `UserConstructionScript`)