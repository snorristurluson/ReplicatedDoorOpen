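; A replicated door actor that swings smoothly between closed and open by rotating its Door component 90 degrees in yaw.
; Open and Close drive a four-state machine and the DoorMovement timeline, which can reverse mid-swing and settles the State when finished.
; OnRep_State calls AnimateDoor, which plays a separate ClientDoorAnimation timeline locally or snaps to the end pose, so only State, rather than rotation, drives client visuals.
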(event `/Game/Blueprints/Openable.Open`
  (switch `/Game/Blueprints/EDoorState` (`self.State`)
    (:`NewEnumerator0`
      (set `self.State` "NewEnumerator1")
      (bind (_direction _value) (`Timeline|DoorMovement` :!via `PlayFromStart` :!label _label)
        (:`Update`
          (`self.Update Door State` _value))
        (:`Finished`
          (set `self.State` (select `ETimelineDirection` _direction :`Forward` "NewEnumerator2" :`Backward` "NewEnumerator0" :!type "/Game/Blueprints/EDoorState Enum")))))
    (:`NewEnumerator1`
      (goto _label))
    (:`NewEnumerator3`
      (set `self.State` "NewEnumerator1")
      (goto _label))))

(event `/Game/Blueprints/Openable.Close`
  (switch `/Game/Blueprints/EDoorState` (`self.State`)
    (:`NewEnumerator1`
      (set `self.State` "NewEnumerator3")
      (goto _label :!via `Reverse`))
    (:`NewEnumerator2`
      (set `self.State` "NewEnumerator3")
      (goto _label :!via `ReverseFromEnd`))
    (:`NewEnumerator3`
      (goto _label :!via `Reverse`))))

(event `Animate Door`
  (switch `/Game/Blueprints/EDoorState` (`self.State`)
    (:`NewEnumerator0`
      (`TimelineComponent.Stop` (`self.ClientDoorAnimation`))
      (`self.Update Door State` 0.0))
    (:`NewEnumerator1`
      (bind (_direction _value) (`Timeline|ClientDoorAnimation` :!via `PlayFromStart` :!label _label_2)
        (:`Update`
          (`self.Update Door State` _value))))
    (:`NewEnumerator2`
      (`TimelineComponent.Stop` (`self.ClientDoorAnimation`))
      (`self.Update Door State` 1.0))
    (:`NewEnumerator3`
      (goto _label_2 :!via `ReverseFromEnd`))))

(fn `OnRep_State`
  (`self.Animate Door`))

(fn `Update Door State`
  (params (Value :type "Float (double-precision)"))
  (`SceneComponent.K2_SetRelativeRotation` (`self.Door`) (`KismetMathLibrary.MakeRotator` 0.0 0.0 (* Value 90.0)) false false))

(fn `UserConstructionScript`)